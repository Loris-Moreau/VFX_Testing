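; Weeping Angel enemy that advances on the player while unseen and freezes when on screen.
; After a start delay, a self-repeating short-delay loop checks whether the mesh was recently rendered.
; When rendered, it stops movement and zeroes the animation rate; otherwise it restores animation and uses simple navigation toward the player's current location.
; Any actor that begins overlapping it takes a random amount of damage.
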(event Custom|Silent_Assasin_Move
  ;[1 0.6425 0.35] Weeping Angels
  (if (Class|PrimitiveComponent|WasRecentlyRendered (Variables|Character|GetMesh) 0.04)
    (if (Variables|Default|GetIsMoving)
      (Components|Movement|StopMovementImmediately (Variables|Character|GetCharacterMovement))
      (Variables|Default|SetIsMoving false)
      (Variables|/Script/Engine.SkeletalMeshComponent|SetGlobalAnimRateScale (Variables|Character|GetMesh) 0.0))
    (else
      (AI|Navigation|SimpleMovetoLocation (Pawn|GetController) (Transformation|GetActorLocation (Game|GetPlayerCharacter 0)))
      (Variables|Default|SetIsMoving true)
      (Variables|/Script/Engine.SkeletalMeshComponent|SetGlobalAnimRateScale (Variables|Character|GetMesh) 1.0)))
  (Utilities|FlowControl|Delay 0.01)
  (CallFunction|SilentAssasinMove))

(event Collision|EventActorBeginOverlap
  (params (OtherActor :type Actor%20Object%20Reference))
  (Game|Damage|ApplyDamage OtherActor (Math|Random|RandomFloatinRange 5.0 15.0) 0 self "/Script/Engine.DamageType"))

(event EventBeginPlay
  (Utilities|FlowControl|Delay 1e+01)
  (CallFunction|SilentAssasinMove))

(fn ConstructionScript)