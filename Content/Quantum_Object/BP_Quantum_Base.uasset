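; Base Blueprint for a quantum object that jumps to another location when it leaves the player's view.
; A self-recalling Delay loop polls WasRecentlyRendered from BeginPlay and triggers one relocation attempt on each visible-to-hidden change.
; FindNewLocation draws randomly from QuantumLocations, discarding the current spot and visible candidates until one qualifies or none remain.
; The actor teleports to the chosen spot, or stays put if none qualifies.
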(event Custom|Check%20Visibility
  (if (Class|Actor|WasRecentlyRendered 0.1)
    (Variables|Default|SetIsVisible true)
    (elif (Variables|Default|GetIsVisible)
      (Variables|Default|SetIsVisible false)
      (bind (_location _canteleport) (CallFunction|FindNewLocation))
      (if _canteleport
        (Transformation|SetActorLocation _location false false))))
  (Utilities|FlowControl|Delay 0.001)
  (CallFunction|CheckVisibility))

(event EventBeginPlay
  (CallFunction|CheckVisibility))

(fn ConstructionScript)

(fn FindNewLocation
  (bind _output_get (LocalVariables|SetTemp%20Location (Variables|Default|GetQuantum%20Locations)))
  (if (== (Utilities|Array|Length _output_get) 0) :!label _label
    (return "0, 0, 0" false)
    (else
      (LocalVariables|SetCurrent%20Index (Math|Random|RandomIntegerinRange 0 (- (Utilities|Array|Length _output_get) 1)))
      (if (Utilities|Operators|NotEqual(!=) (Transformation|GetActorLocation (Utilities|Array|Get(acopy) (LocalVariables|GetTemp%20Location) (LocalVariables|GetCurrent%20Index))) (Transformation|GetActorLocation) 5.0)
        (if (Variables|/Game/Quantum_Object/BP_Quantum_Spawn.BP_Quantum_Spawn_C|GetIsVisible (Utilities|Array|Get(acopy) (LocalVariables|GetTemp%20Location) (LocalVariables|GetCurrent%20Index)))
          _
          (else
            (return (Transformation|GetActorLocation (Utilities|Array|Get(acopy) (LocalVariables|GetTemp%20Location) (LocalVariables|GetCurrent%20Index))) true))))
      (Utilities|Array|RemoveIndex (LocalVariables|GetTemp%20Location) (LocalVariables|GetCurrent%20Index))
      (goto _label))))