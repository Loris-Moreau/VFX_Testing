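; BP_DiscoLight is a Blueprint that endlessly cycles a point light through four colors for a disco effect.
; BeginPlay starts a self-looping chain on a short retriggerable delay, with each color change wired back into the delay.
; Nested FlipFlops act as a four-step sequencer, alternating between two pairs so the light runs yellow, green, red, then blue.
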(event EventBeginPlay
  (bind _pointlight (Variables|Default|GetPointLight))
  (Utilities|FlowControl|RetriggerableDelay 0.2 :!label _label)
  (Utilities|FlowControl|FlipFlop
    (:A
      (Utilities|FlowControl|FlipFlop
        (:A
          (Rendering|Components|Light|SetLightColor _pointlight (Class|KismetMathLibrary|LinearColorYellow) true)
          (goto _label))
        (:B
          (Rendering|Components|Light|SetLightColor _pointlight (Class|KismetMathLibrary|LinearColorRed) true)
          (goto _label))))
    (:B
      (Utilities|FlowControl|FlipFlop
        (:A
          (Rendering|Components|Light|SetLightColor _pointlight (Class|KismetMathLibrary|LinearColorGreen) true)
          (goto _label))
        (:B
          (Rendering|Components|Light|SetLightColor _pointlight (Class|KismetMathLibrary|LinearColorBlue) true)
          (goto _label))))))

(fn ConstructionScript)