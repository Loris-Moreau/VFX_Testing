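; BP_ComicLight is a lighting driver for the stylized comic shader, feeding light data into a Material Parameter Collection.
; Every Tick it writes the front and back rim colors and the directional light's forward vector, converted to a color, as named vector parameters.
; The construction script is empty, and a few unnamed parameter writes are left unconnected.
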(event EventTick
  (params (DeltaSeconds :type Float%20%28single-precision%29))
  (Rendering|Material|SetVectorParameterValue (Variables|References|GetMPC) (Variables|Name|GetRim%20Front%20Name) (Variables|Color|GetRim%20Front%20Color) :!class /Script/Engine.KismetMaterialLibrary)
  (Rendering|Material|SetVectorParameterValue (Variables|References|GetMPC) (Variables|Name|GetRim%20Back%20Name) (Variables|Color|GetRim%20Back%20Color) :!class /Script/Engine.KismetMaterialLibrary)
  (Rendering|Material|SetVectorParameterValue (Variables|References|GetMPC) (Variables|Name|GetLight%20Direction%20Name) (Math|Conversions|ToLinearColor(Vector) (Math|Vector|GetForwardVector (Variables|Default|GetDirectionalLight))) :!class /Script/Engine.KismetMaterialLibrary))

(fn ConstructionScript)