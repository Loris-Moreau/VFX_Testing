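; Audio visualizer actor that plays a sound and spawns bar-like BP_AudioElement actors scaled by its frequency spectrum.
; It takes the sound from a ConstantQ analysis asset and converts each playback-percent callback into a time in seconds.
; It loops over channel 0's normalized Constant-Q values at that time, with a short Delay before spawning at the root location.
; Each value times HeightMultiplier sets the spawned element's Z scale.
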(event Custom|PlaybackChange
  (params (PlayingSoundWave :type Sound%20Wave%20Object%20Reference) (PlaybackPercent :type Float%20%28single-precision%29))
  (bind _output_get (Variables|Default|SetPlayerTime (* PlaybackPercent (Variables|Default|GetDuration))))
  (for _array_element (Class|ConstantQNRT|GetNormalizedChannelConstantQatTime (Variables|Default|GetConstant%20Ref) _output_get)
    (Utilities|FlowControl|Delay 0.05)
    (Game|SpawnActorfromClass "/Game/VFX/AudioWave/BP_AudioElement.BP_AudioElement_C" (Math|Transform|MakeTransform (Transformation|GetWorldLocation (Variables|Default|GetDefaultSceneRoot)) "0, 0, 0" (Math|Vector|MakeVector 0.15 0.15 (* _array_element (Variables|Default|GetHeight%20Multiplier)))) "Undefined" "MultiplyWithRoot" 0 0)))

(event EventBeginPlay
  (Variables|Default|SetSound (Variables|/Script/AudioAnalyzer.AudioAnalyzerNRT|GetSound (Variables|Default|GetConstant%20Ref)))
  (Audio|Components|Audio|SetSound (Variables|Default|GetAudio) (Variables|Default|GetSound))
  (Variables|Default|SetDuration (Variables|/Script/Engine.SoundBase|GetDuration (Variables|Default|GetSound)))
  (EventDispatchers|BindEventtoOnAudioPlaybackPercent (Variables|Default|GetAudio) (delegate Custom|PlaybackChange))
  (Audio|Components|Audio|Play (Variables|Default|GetAudio) 0.0))

(fn ConstructionScript)