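; BP_Slime2 is a slime character that feeds its movement state to the materials on its Slime component.
; On BeginPlay it starts MoveSlime, a self-calling event that repeats every tenth of a second without using Tick.
; Each pass writes scaled movement velocity to the RotAxis vector parameter and the component's forward vector to ForwardVector, leaving any visual response to the materials.
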(event Custom|MoveSlime
  (Rendering|Material|SetVectorParameterValueonMaterials (Variables|Default|GetSlime) "RotAxis" (/ (Variables|/Script/Engine.MovementComponent|GetVelocity (Variables|Character|GetCharacterMovement)) 1e+02))
  (Rendering|Material|SetVectorParameterValueonMaterials (Variables|Default|GetSlime) "ForwardVector" (Math|Vector|GetForwardVector (Variables|Default|GetSlime)))
  (Utilities|FlowControl|Delay 0.1)
  (CallFunction|MoveSlime))

(event EventBeginPlay
  (CallFunction|MoveSlime))

(fn ConstructionScript)